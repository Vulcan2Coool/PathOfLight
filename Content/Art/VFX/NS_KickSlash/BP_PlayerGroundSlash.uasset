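; Short-lived player ground slash attack actor that plays sounds on spawn, damages enemies and breaks destructibles.
; Each Tick it sphere-traces between two components and branches on object type, applying reduced damage to bosses and skipping actors already hit.
; Hits spawn punch VFX and raise the player's combo once per branch, also feeding the GameInstance.
; Destructibles fracture through Chaos strain, and world static, crit spots or the first break destroy the slash.
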(event OnComponentBeginOverlap(GS_Collider)
  (params (OverlappedComponent :type Primitive%20Component%20Object%20Reference) (OtherActor :type Actor%20Object%20Reference) (OtherComp :type Primitive%20Component%20Object%20Reference) (OtherBodyIndex :type Integer) (bFromSweep :type Boolean) (SweepResult :type Hit%20Result%20Structure%20%28by%20ref%29)))

(event Custom|Increment%20Combo
  (params (amt :type Float%20%28double-precision%29))
  (bind _asbp_game_instance (Utilities|Casting|CastToBP_GameInstance (Game|GetGameInstance)))
  (Variables|/Game/Blueprints/BP_GameInstance.BP_GameInstance_C|SetPlayCombo _asbp_game_instance (+ (Variables|/Game/Blueprints/BP_GameInstance.BP_GameInstance_C|GetPlayCombo _asbp_game_instance) amt)))

(event EventBeginPlay
  (bind _returnvalue (Math|Random|RandomFloatinRange 0.7 1.2))
  (bind _self self)
  (bind _returnvalue_2 (Transformation|GetActorLocation _self))
  (bind _asbase_character (Utilities|Casting|CastToBase_Character (Game|GetPlayerCharacter 0)))
  (Variables|Default|SetAs%20Base%20Character _asbase_character)
  (Audio|PlaySoundatLocation "/Game/Art/SFX/InGame/closeup-sting.closeup-sting" _returnvalue_2 "0, 0, 0" 0.6 _returnvalue 0.0 0 0 0 0)
  (Audio|PlaySoundatLocation "/Game/Art/SFX/InGame/SW_Woosh4.SW_Woosh4" _returnvalue_2 "0, 0, 0" 1.0 _returnvalue 0.0 0 0 0 0)
  (Audio|PlaySoundatLocation "/Game/Art/SFX/UI_SFX/quake-and-break-99034.quake-and-break-99034" _returnvalue_2 "0, 0, 0" 2.0 _returnvalue 3.0 0 0 0 0)
  (Actor|SetLifeSpan 3.0))

(event EventTick
  (params (DeltaSeconds :type Float%20%28single-precision%29))
  (bind _as_base_character (Variables|Default|GetAs%20Base%20Character))
  (bind _as_base_character_2 (Variables|Default|GetAs%20Base%20Character))
  (Variables|Default|SetTimer DeltaSeconds)
  (bind _outhits (Collision|MultiSphereTraceForObjects (Transformation|GetWorldLocation (Variables|Default|GetStart)) (Transformation|GetWorldLocation (Variables|Default|GetEnd)) 5e+01 (Utilities|Array|MakeArray "ObjectTypeQuery6" "ObjectTypeQuery14" "ObjectTypeQuery3" "ObjectTypeQuery18" "ObjectTypeQuery12") false 0 "None"))
  (for _array_element _outhits
    (if (not (Utilities|Array|ContainsItem (Variables|Default|GetActorsToIgnore) (.hitactor _array_element)))
      (switch Utilities|FlowControl|Switch|SwitchonECollisionChannel (Collision|GetCollisionObjectType (.hitcomponent _array_element))
        (:ECC_WorldStatic
          (Actor|DestroyActor))
        (:ECC_Pawn
          (Niagara|SpawnSystematLocation "/Game/Art/VFX/NS_Punch.NS_Punch" (.impactpoint _array_element))
          (Game|Damage|ApplyDamage (.hitactor _array_element) (Variables|Default|GetDamage%20Variable) (Game|GetPlayerController 0) _as_base_character_2 "/Game/Blueprints/Damaging/DT_PlayerLightAttack.DT_PlayerLightAttack_C")
          (Utilities|Array|Add (Variables|Default|GetActorsToIgnore) (.hitactor _array_element))
          (Utilities|FlowControl|DoOnce false
            (:Completed
              (Variables|/Game/Blueprints/Characters/Base_Character.Base_Character_C|SetComboCount _as_base_character_2 (+ (Variables|/Game/Blueprints/Characters/Base_Character.Base_Character_C|GetComboCount _as_base_character_2) 2.0))
              (CallFunction|IncrementCombo (+ (Variables|/Game/Blueprints/Characters/Base_Character.Base_Character_C|GetComboCount _as_base_character_2) 2.0))
              (Default|IncrementComboAch _as_base_character_2 2))))
        (:ECC_Destructible
          (bind _aschaos_parent (Utilities|Casting|CastToChaos_Parent (.hitactor _array_element)))
          (bind _output_get (Variables|/Game/Blueprints/Destruction/Chaos_Parent.Chaos_Parent_C|SetDestructionCenter _aschaos_parent (.impactpoint _array_element)))
          (bind _asgeometry_collection_component (Utilities|Casting|CastToGeometryCollectionComponent (.hitcomponent _array_element)))
          (Class|GeometryCollectionComponent|ApplyInternalStrain _asgeometry_collection_component (.hititem _array_element) _output_get 1e+02 0 1.0 1e+08)
          (if (not (Variables|Default|GetSoundBreak))
            (Utilities|FlowControl|DoOnce false
              (:Completed
                (Audio|PlaySound2D "/Game/Art/SFX/InGame/ER_WoodBreaking.ER_WoodBreaking" 1.0 1.0 0.0 0 0)
                (Variables|Default|SetSoundBreak true)
                (Utilities|FlowControl|Delay 0.1)
                (Actor|DestroyActor)))))
        (:ECC_GameTraceChannel8
          (Niagara|SpawnSystematLocation "/Game/Art/VFX/NS_Punch.NS_Punch" (.impactpoint _array_element) :!label _label)
          (Utilities|Casting|CastToBP_Base_Boss (.hitactor _array_element))
          (Game|Damage|ApplyDamage (.hitactor _array_element) (Math|Conversions|ToFloat(Integer) (Math|Float|Round (* (Variables|Default|GetDamage%20Variable) 0.85))) 0 _as_base_character)
          (Utilities|Array|Add (Variables|Default|GetActorsToIgnore) (.hitactor _array_element))
          (Utilities|FlowControl|DoOnce false
            (:Completed
              (Variables|/Game/Blueprints/Characters/Base_Character.Base_Character_C|SetComboCount _as_base_character (+ (Variables|/Game/Blueprints/Characters/Base_Character.Base_Character_C|GetComboCount _as_base_character) 4.0))
              (CallFunction|IncrementCombo (+ (Variables|/Game/Blueprints/Characters/Base_Character.Base_Character_C|GetComboCount _as_base_character) 4.0))
              (Default|IncrementComboAch _as_base_character 4))))
        (:ECC_GameTraceChannel10
          (Actor|DestroyActor))
        (:ECC_GameTraceChannel14
          (goto _label))))))

(fn ConstructionScript)