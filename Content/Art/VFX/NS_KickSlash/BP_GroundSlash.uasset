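; Ground slash projectile that damages characters and can be deflected, with a three-second lifespan.
; On spawn it plays sting, whoosh and quake sounds at random pitch; its terrain collider destroys it on any overlap.
; Its hit collider damages overlapped Base_Character actors, or reverses velocity if they can deflect.
; A DoOnce resets only after damage, so a deflected slash ignores later character overlaps.
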(event OnComponentBeginOverlap(TerrainCollider)
  (params (OverlappedComponent :type Primitive%20Component%20Object%20Reference) (OtherActor :type Actor%20Object%20Reference) (OtherComp :type Primitive%20Component%20Object%20Reference) (OtherBodyIndex :type Integer) (bFromSweep :type Boolean) (SweepResult :type Hit%20Result%20Structure%20%28by%20ref%29))
  (Actor|DestroyActor self))

(event OnComponentBeginOverlap(GS_Collider)
  (params (OverlappedComponent :type Primitive%20Component%20Object%20Reference) (OtherActor :type Actor%20Object%20Reference) (OtherComp :type Primitive%20Component%20Object%20Reference) (OtherBodyIndex :type Integer) (bFromSweep :type Boolean) (SweepResult :type Hit%20Result%20Structure%20%28by%20ref%29))
  (bind _asbase_character (Utilities|Casting|CastToBase_Character OtherActor))
  (Utilities|FlowControl|DoOnce false :!label _label
    (:Completed
      (if (Variables|/Game/Blueprints/Characters/Base_Character.Base_Character_C|GetCanDeflect _asbase_character)
        (Variables|/Script/Engine.MovementComponent|SetVelocity (Variables|Default|GetProjectileMovement) (Math|Vector|NegateVector (Transformation|GetVelocity)))
        (else
          (Game|Damage|ApplyDamage _asbase_character 3e+01 0 (Components|GetOwner (Variables|Default|GetGroundSLash)))
          (goto _label Reset))))))

(event EventBeginPlay
  (bind _returnvalue (Math|Random|RandomFloatinRange 0.7 1.2))
  (bind _self self)
  (bind _returnvalue_2 (Transformation|GetActorLocation _self))
  (Audio|PlaySoundatLocation "/Game/Art/SFX/InGame/closeup-sting.closeup-sting" _returnvalue_2 "0, 0, 0" 0.6 _returnvalue 0.0 0 0 0 0)
  (Audio|PlaySoundatLocation "/Game/Art/SFX/InGame/SW_Woosh4.SW_Woosh4" _returnvalue_2 "0, 0, 0" 1.0 _returnvalue 0.0 0 0 0 0)
  (Audio|PlaySoundatLocation "/Game/Art/SFX/UI_SFX/quake-and-break-99034.quake-and-break-99034" _returnvalue_2 "0, 0, 0" 2.0 _returnvalue 3.0 0 0 0 0)
  (Actor|SetLifeSpan 3.0))

(fn ConstructionScript)