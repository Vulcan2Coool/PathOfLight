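; Player finisher attack actor for Cyrus that launches five ground-slash colliders along their forward vectors, with sounds and a short lifespan.
; Each slash collider damages overlapped actors that are not Base_Character, then triggers the player's finisher health restore.
; Terrain colliders drop their attach parent far below the world on overlap, removing that slash from play.
; The player reference is not assigned in any executed path here.
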(event OnComponentBeginOverlap(GS_Collider2)
  (params (OverlappedComponent :type Primitive%20Component%20Object%20Reference) (OtherActor :type Actor%20Object%20Reference) (OtherComp :type Primitive%20Component%20Object%20Reference) (OtherBodyIndex :type Integer) (bFromSweep :type Boolean) (SweepResult :type Hit%20Result%20Structure%20%28by%20ref%29))
  (bind _as_bp_cyrus_player (Variables|Default|GetAs%20BP%20Cyrus%20Player))
  (Utilities|Casting|CastToBase_Character OtherActor
    (:CastFailed
      (Utilities|FlowControl|DoOnce false :!label _label
        (:Completed
          (Game|Damage|ApplyDamage OtherActor (Variables|Default|GetBase%20Damage) (Pawn|GetController _as_bp_cyrus_player) _as_bp_cyrus_player)
          (CallFunction|LocalEventFinisherHeals)
          (goto _label Reset))))))

(event OnComponentBeginOverlap(GS_Collider)
  (params (OverlappedComponent :type Primitive%20Component%20Object%20Reference) (OtherActor :type Actor%20Object%20Reference) (OtherComp :type Primitive%20Component%20Object%20Reference) (OtherBodyIndex :type Integer) (bFromSweep :type Boolean) (SweepResult :type Hit%20Result%20Structure%20%28by%20ref%29))
  (Utilities|Casting|CastToBase_Character OtherActor
    (:CastFailed
      (Utilities|FlowControl|DoOnce false :!label _label
        (:Completed
          (Game|Damage|ApplyDamage OtherActor (Variables|Default|GetBase%20Damage) (Game|GetPlayerController 0) (Variables|Default|GetAs%20BP%20Cyrus%20Player))
          (CallFunction|LocalEventFinisherHeals)
          (goto _label Reset))))))

(event OnComponentBeginOverlap(GS_Collider1)
  (params (OverlappedComponent :type Primitive%20Component%20Object%20Reference) (OtherActor :type Actor%20Object%20Reference) (OtherComp :type Primitive%20Component%20Object%20Reference) (OtherBodyIndex :type Integer) (bFromSweep :type Boolean) (SweepResult :type Hit%20Result%20Structure%20%28by%20ref%29))
  (bind _as_bp_cyrus_player (Variables|Default|GetAs%20BP%20Cyrus%20Player))
  (Utilities|Casting|CastToBase_Character OtherActor
    (:CastFailed
      (Utilities|FlowControl|DoOnce false :!label _label
        (:Completed
          (Game|Damage|ApplyDamage OtherActor (Variables|Default|GetBase%20Damage) (Pawn|GetController _as_bp_cyrus_player) _as_bp_cyrus_player)
          (CallFunction|LocalEventFinisherHeals)
          (goto _label Reset))))))

(event OnComponentBeginOverlap(TerrainCollider1)
  (params (OverlappedComponent :type Primitive%20Component%20Object%20Reference) (OtherActor :type Actor%20Object%20Reference) (OtherComp :type Primitive%20Component%20Object%20Reference) (OtherBodyIndex :type Integer) (bFromSweep :type Boolean) (SweepResult :type Hit%20Result%20Structure%20%28by%20ref%29))
  (bind _returnvalue (Transformation|GetAttachParent OverlappedComponent))
  (Utilities|IsValid _returnvalue
    (:Is%20Valid
      (Transformation|AddWorldOffset _returnvalue "0.000000,0.000000,-9999.000000" false false))))

(event OnComponentBeginOverlap(TerrainCollider2)
  (params (OverlappedComponent :type Primitive%20Component%20Object%20Reference) (OtherActor :type Actor%20Object%20Reference) (OtherComp :type Primitive%20Component%20Object%20Reference) (OtherBodyIndex :type Integer) (bFromSweep :type Boolean) (SweepResult :type Hit%20Result%20Structure%20%28by%20ref%29))
  (bind _returnvalue (Transformation|GetAttachParent OverlappedComponent))
  (Utilities|IsValid _returnvalue
    (:Is%20Valid
      (Transformation|AddWorldOffset _returnvalue "0.000000,0.000000,-9999.000000" false false))))

(event OnComponentBeginOverlap(TerrainCollider)
  (params (OverlappedComponent :type Primitive%20Component%20Object%20Reference) (OtherActor :type Actor%20Object%20Reference) (OtherComp :type Primitive%20Component%20Object%20Reference) (OtherBodyIndex :type Integer) (bFromSweep :type Boolean) (SweepResult :type Hit%20Result%20Structure%20%28by%20ref%29))
  (bind _returnvalue (Transformation|GetAttachParent OverlappedComponent))
  (Utilities|IsValid _returnvalue
    (:Is%20Valid
      (Transformation|AddWorldOffset _returnvalue "0.000000,0.000000,-9999.000000" false false))))

(event OnComponentBeginOverlap(GS_Collider3)
  (params (OverlappedComponent :type Primitive%20Component%20Object%20Reference) (OtherActor :type Actor%20Object%20Reference) (OtherComp :type Primitive%20Component%20Object%20Reference) (OtherBodyIndex :type Integer) (bFromSweep :type Boolean) (SweepResult :type Hit%20Result%20Structure%20%28by%20ref%29))
  (bind _as_bp_cyrus_player (Variables|Default|GetAs%20BP%20Cyrus%20Player))
  (Utilities|Casting|CastToBase_Character OtherActor
    (:CastFailed
      (Utilities|FlowControl|DoOnce false :!label _label
        (:Completed
          (Game|Damage|ApplyDamage OtherActor (Variables|Default|GetBase%20Damage) (Pawn|GetController _as_bp_cyrus_player) _as_bp_cyrus_player)
          (CallFunction|LocalEventFinisherHeals)
          (goto _label Reset))))))

(event OnComponentBeginOverlap(GS_Collider4)
  (params (OverlappedComponent :type Primitive%20Component%20Object%20Reference) (OtherActor :type Actor%20Object%20Reference) (OtherComp :type Primitive%20Component%20Object%20Reference) (OtherBodyIndex :type Integer) (bFromSweep :type Boolean) (SweepResult :type Hit%20Result%20Structure%20%28by%20ref%29))
  (bind _as_bp_cyrus_player (Variables|Default|GetAs%20BP%20Cyrus%20Player))
  (Utilities|Casting|CastToBase_Character OtherActor
    (:CastFailed
      (Utilities|FlowControl|DoOnce false :!label _label
        (:Completed
          (Game|Damage|ApplyDamage OtherActor (Variables|Default|GetBase%20Damage) (Pawn|GetController _as_bp_cyrus_player) _as_bp_cyrus_player)
          (CallFunction|LocalEventFinisherHeals)
          (goto _label Reset))))))

(event OnComponentBeginOverlap(TerrainCollider3)
  (params (OverlappedComponent :type Primitive%20Component%20Object%20Reference) (OtherActor :type Actor%20Object%20Reference) (OtherComp :type Primitive%20Component%20Object%20Reference) (OtherBodyIndex :type Integer) (bFromSweep :type Boolean) (SweepResult :type Hit%20Result%20Structure%20%28by%20ref%29))
  (bind _returnvalue (Transformation|GetAttachParent OverlappedComponent))
  (Utilities|IsValid _returnvalue
    (:Is%20Valid
      (Transformation|AddWorldOffset _returnvalue "0.000000,0.000000,-9999.000000" false false))))

(event OnComponentBeginOverlap(TerrainCollider4)
  (params (OverlappedComponent :type Primitive%20Component%20Object%20Reference) (OtherActor :type Actor%20Object%20Reference) (OtherComp :type Primitive%20Component%20Object%20Reference) (OtherBodyIndex :type Integer) (bFromSweep :type Boolean) (SweepResult :type Hit%20Result%20Structure%20%28by%20ref%29))
  (bind _returnvalue (Transformation|GetAttachParent OverlappedComponent))
  (Utilities|IsValid _returnvalue
    (:Is%20Valid
      (Transformation|AddWorldOffset _returnvalue "0.000000,0.000000,-9999.000000" false false))))

(event Custom|localEvent%20FinisherHeals
  (bind _as_bp_cyrus_player (Variables|Default|GetAs%20BP%20Cyrus%20Player))
  (Variables|/Game/Blueprints/Characters/Base_Character.Base_Character_C|SetFinisher _as_bp_cyrus_player true)
  (Variables|/Game/Blueprints/Characters/Base_Character.Base_Character_C|SetOnHit _as_bp_cyrus_player true)
  (Default|BCFinisherRestoreHealth _as_bp_cyrus_player))

(event EventBeginPlay
  (bind _returnvalue (Math|Random|RandomFloatinRange 0.7 1.2))
  (bind _self self)
  (bind _gs_collider1 (Variables|Default|GetGS_Collider1))
  (bind _gs_collider2 (Variables|Default|GetGS_Collider2))
  (bind _gs_collider (Variables|Default|GetGS_Collider))
  (bind _gs_collider4 (Variables|Default|GetGS_Collider4))
  (bind _gs_collider3 (Variables|Default|GetGS_Collider3))
  (bind _returnvalue_2 (Transformation|GetActorLocation _self))
  (Variables|/Game/Blueprints/Characters/Base_Character.Base_Character_C|SetFinisher (Variables|Default|GetAs%20BP%20Cyrus%20Player) true)
  (Audio|PlaySoundatLocation "/Game/Art/SFX/InGame/closeup-sting.closeup-sting" _returnvalue_2 "0, 0, 0" 0.6 _returnvalue 0.0 0 0 0 0)
  (Audio|PlaySoundatLocation "/Game/Art/SFX/InGame/SW_Woosh4.SW_Woosh4" _returnvalue_2 "0, 0, 0" 1.0 _returnvalue 0.0 0 0 0 0)
  (Audio|PlaySoundatLocation "/Game/Art/SFX/UI_SFX/quake-and-break-99034.quake-and-break-99034" _returnvalue_2 "0, 0, 0" 2.0 _returnvalue 3.0 0 0 0 0)
  (Physics|AddImpulse _gs_collider1 (* (Math|Vector|GetForwardVector _gs_collider1) 3e+03) "None" true)
  (Physics|AddImpulse _gs_collider2 (* (Math|Vector|GetForwardVector _gs_collider2) 3e+03) "None" true)
  (Physics|AddImpulse _gs_collider (* (Math|Vector|GetForwardVector _gs_collider) 3e+03) "None" true)
  (Physics|AddImpulse _gs_collider4 (* (Math|Vector|GetForwardVector _gs_collider4) 3e+03) "None" true)
  (Physics|AddImpulse _gs_collider3 (* (Math|Vector|GetForwardVector _gs_collider3) 3e+03) "None" true)
  (Actor|SetLifeSpan 2.5))

(fn ConstructionScript)