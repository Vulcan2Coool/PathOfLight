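; BP_Western_Boss is the Cyrus boss enemy, with a separate health and phase setup for the Boss Rush level.
; Accumulated damage advances phases and writes special or state enums to the Blackboard.
; Montage attacks fire end dispatchers, while Tick runs socket-based hit traces from fist and leg flags.
; It also dashes to retried random navigable points around the player, shows random subtitle lines on a timer and handles death.
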(event Custom|VA%20loop
  ;[1 1 1] voice lines
  (Utilities|Time|SetTimerbyEvent (delegate Custom|choose%20random%20line) 2e+01 true false -3.0))

(event Custom|choose%20random%20line
  ;[1 1 1] voice lines
  (if (== (Math|Random|RandomIntegerinRange 0 1) 1)
    (bind _returnvalue (UserInterface|CreateWidget "/Game/Blueprints/UI/VA/WBP_BossSubtitles.WBP_BossSubtitles_C" (Game|GetPlayerController 0) (.OutItem (Utilities|Array|Random (Variables|Default|GetVA%20array)))))
    (UserInterface|Viewport|AddtoViewport _returnvalue 0)))

(event Custom|BossDodge
  (bind _mesh (Variables|Character|GetMesh))
  ;[1 1 1] Random location in ring around actor, retry 10 times
  (Utilities|FlowControl|Sequence
    (:then_0
      (bind (_return_value _randomlocation) (CallFunction|RandomNavigatablePointinRing (Transformation|GetActorLocation (Variables|Default|GetBase%20Char%20Ref)) 1e+03 :!label _label))
      (if _return_value
        ;[0.8808 1 0.1927] Dodge
        (Variables|Default|SetInitialDodgeLocation (Transformation|GetActorLocation))
        (Variables|Default|SetChosenDodgeLocation _randomlocation)
        (CallFunction|MontageReplicationRPC "/Game/Art/Characters/Enemies/WesternBoss/Animations/Monmtages/AM_CyrusRun.AM_CyrusRun" 2.0 "None" 0 _mesh 0.0 true)
        (Animation|Montage|PlayMontage _mesh "/Game/Art/Characters/Enemies/WesternBoss/Animations/Monmtages/AM_CyrusRun.AM_CyrusRun" 2.0
          (:then
            (Utilities|FlowControl|Delay 0.2)
            (Audio|PlaySound2D "/Game/Art/SFX/InGame/SW_WooshSlow5.SW_WooshSlow5" 0.8 0.8 0.0 0 0)
            (Niagara|SpawnSystematLocation "/Game/Art/VFX/NS_Dash.NS_Dash" "0, 0, 0")
            (bind _alpha (Timeline|Timeline PlayFromStart)
              (:Update
                (Transformation|SetActorLocation (Math|Vector|MakeVector (.x (Math|Vector|Lerp(Vector) (Variables|Default|GetInitialDodgeLocation) (Variables|Default|GetChosenDodgeLocation) _alpha)) (.y (Math|Vector|Lerp(Vector) (Variables|Default|GetInitialDodgeLocation) (Variables|Default|GetChosenDodgeLocation) _alpha)) (.z (Transformation|GetActorLocation (Variables|Default|GetBase%20Char%20Ref)))) false false))
              (:Finished
                (Default|CallDashDispatch :!label _label_2)))))
        (else
          (Utilities|DoNThenBranch 10 :!label _label_3
            (:Exit
              (goto _label))
            (:Branch
              (goto _label_2))))))
    (:then_1
      (goto _label_3 Reset))))

(event Game|Damage|EventAnyDamage
  (params (Damage :type Float%20%28single-precision%29) (DamageType :type Damage%20Type%20Object%20Reference) (InstigatedBy :type Controller%20Object%20Reference) (DamageCauser :type Actor%20Object%20Reference))
  (bind _isbossrush (Variables|Default|GetIsBossRush))
  ;[1 0.417 0.2768] Damage Boss & Set Run away State
  (Audio|PlaySoundatLocation "/Game/Art/SFX/RandomHitCue.RandomHitCue" (Transformation|GetActorLocation) "0, 0, 0" 1.0 (Math|Random|RandomFloatinRange 0.5 1.3) 0.0 0 0 0 0)
  (if true
    ;;[1 1 1] show dmg numbers?
    (bind _dmgtoapply (CallFunction|DmgNums Damage)))
  (bind _asbase_character (Utilities|Casting|CastToBase_Character DamageCauser))
  (if (Variables|/Game/Blueprints/Characters/Base_Character.Base_Character_C|GetSyd _asbase_character)
    ;;[1 1 1] is dmg causer syd
    (AddComponent|AddNiagaraComponent false))
  (bind _output_get (Variables|Default|SetHealth (- (Variables|Default|GetHealth) _dmgtoapply)))
  (Variables|Default|SetParent%20Boss%20Health _output_get)
  (if (<= _output_get 0.0)
    (CallFunction|OnDeathCustomEvent "/Game/Art/Characters/Enemies/WesternBoss/Animations/Monmtages/AM_CyrusDeath.AM_CyrusDeath" "/Game/Blueprints/UI/VA/dataTables/cyrus/DT_CyrusDeath.DT_CyrusDeath" (Variables|Character|GetMesh) self _isbossrush (Variables|Default|GetBase%20Char%20Ref))
    (Utilities|FlowControl|DoOnce false
      (:Completed
        (Utilities|FlowControl|Delay 2.0)
        (Actor|DestroyActor)))
    (elif _isbossrush
      (bind _output_get_2 (Variables|Default|SetDamageAccumulation (+ _dmgtoapply (Variables|Default|GetDamageAccumulation))))
      (if (>= _output_get_2 (Variables|Default|GetPhaseThreshold))
        (Variables|Default|SetDamageAccumulation 0.0)
        (Variables|Default|SetPhaseThreshold 1e+02)
        (AI|Components|Blackboard|SetValueasEnum (AI|GetBlackboard 0) (Variables|Default|GetSpecialKey) (Utilities|Enum|LiteralenumBossSpecial "NewEnumerator1")))
      (else
        (if (<= _output_get 94.5)
          (Variables|Default|SetIsFinal true))
        (if (or (== (Variables|Default|GetPhaseInt) 4) (Variables|Default|GetIsFinal))
          (AI|Components|Blackboard|SetValueasEnum (AI|GetBlackboard 0) (Variables|Default|GetKeyName) (Utilities|Enum|LiteralenumLightEnemy "NewEnumerator7"))
          (switch int (Variables|Default|GetStunTPInt)
            (:0
              (Variables|Default|SetStunTPInt 1))
            (:1
              (Variables|Default|SetStunTPInt 0)))
          (else
            (bind _output_get_3 (Variables|Default|SetDamageAccumulation (+ _dmgtoapply (Variables|Default|GetDamageAccumulation))))
            (if (>= _output_get_3 (Variables|Default|GetPhaseThreshold))
              (Variables|Default|SetDamageAccumulation 0.0)
              (switch int (Variables|Default|GetPhaseInt)
                (:0
                  (Variables|Default|SetPhaseInt 1)
                  (Variables|Default|SetPhaseThreshold 1.5e+02)
                  (AI|Components|Blackboard|SetValueasEnum (AI|GetBlackboard 0) (Variables|Default|GetSpecialKey) (Utilities|Enum|LiteralenumBossSpecial "NewEnumerator1")))
                (:1
                  (Variables|Default|SetPhaseInt 2)
                  (Variables|Default|SetPhaseThreshold 1.5e+02)
                  (AI|Components|Blackboard|SetValueasEnum (AI|GetBlackboard 0) (Variables|Default|GetSpecialKey) (Utilities|Enum|LiteralenumBossSpecial "NewEnumerator1"))
                  (Variables|Default|SetIsSecond true))
                (:2
                  (Variables|Default|SetPhaseInt 3)
                  (Variables|Default|SetPhaseThreshold 1.5e+02)
                  (AI|Components|Blackboard|SetValueasEnum (AI|GetBlackboard 0) (Variables|Default|GetSpecialKey) (Utilities|Enum|LiteralenumBossSpecial "NewEnumerator1")))
                (:3
                  (Variables|Default|SetPhaseInt 4)
                  (Variables|Default|SetPhaseThreshold 1e+02)
                  (AI|Components|Blackboard|SetValueasEnum (AI|GetBlackboard 0) (Variables|Default|GetSpecialKey) (Utilities|Enum|LiteralenumBossSpecial "NewEnumerator1"))
                  (Variables|Default|SetIsFinal true))
                (:4
                  (AI|Components|Blackboard|SetValueasEnum (AI|GetBlackboard 0) (Variables|Default|GetStateKey) (Utilities|Enum|LiteralenumLightEnemy "NewEnumerator3")))))))))))

(event EventTick
  (params (DeltaSeconds :type Float%20%28single-precision%29))
  ;[1 1 1] Event Tick Line Trace Damage Logic
  (Variables|Default|SetDelta%20Seconds DeltaSeconds)
  (if (Variables|Default|GetShouldRotate)
    (CallFunction|RotateTowardsPlayer))
  (if (Variables|Default|GetLeftFistAttack)
    (Variables|Default|SetSocketStart "LeftHandStart")
    (Variables|Default|SetSocketEnd "LeftHandEnd")
    (CallFunction|AttackTrace (Variables|Character|GetMesh) (Variables|Default|GetSocketStart) (Variables|Default|GetSocketEnd) (Variables|Default|GetDamageCalculator) 5.0 :!label _label)
    (elif (Variables|Default|GetRightFistAttack)
      (Variables|Default|SetSocketStart "RightHandStart")
      (Variables|Default|SetSocketEnd "RightHandEnd")
      (goto _label)
      (elif (Variables|Default|GetHeavyAttack)
        (Variables|Default|SetSocketStart "LeftLegStart")
        (Variables|Default|SetSocketEnd "LeftLegEnd")
        (goto _label)))))

(event EventBeginPlay
  (bind _asbase_character (Utilities|Casting|CastToBase_Character (Game|GetPlayerCharacter 0)))
  (Variables|Default|SetBase%20Char%20Ref _asbase_character)
  (bind _returnvalue (Game|GetCurrentLevelName true))
  (if (Utilities|Enum|Equal(Enum) _returnvalue "LV_BossRush")
    (Variables|Default|SetHealth 4e+02)
    (Variables|Default|SetIsBossRush true)
    (Variables|Default|SetIsSecond true))
  ;[1 1 1] Initialize maxhealth variable for widget
  (Variables|Default|SetParent%20Boss%20Max%20Health (CallFunction|GetNewBossHealth (Variables|Default|GetHealth)))
  (Utilities|FlowControl|Delay 0.2)
  (bind _asbase_character_2 (Utilities|Casting|CastToBase_Character (Game|GetPlayerCharacter 0)))
  (Default|InitCyrusBoss (Variables|/Game/Blueprints/Characters/Base_Character.Base_Character_C|GetHudRef _asbase_character_2))
  (CallFunction|VALoop))

(event Custom|ClearAttackStack
  ;[0.3936 0.9502 1] Clear Stacks From Line Trace
  (Utilities|Array|Clear (Variables|Default|GetActorsToIgnore)))

(event Custom|ChargedKick
  (bind _self self)
  ;[1 0.5847 0.2546] Charged Kick
  (Niagara|SpawnSystematLocation "/Game/Art/VFX/NS_MuzzleFlash.NS_MuzzleFlash" (+ (Math|Vector|GetForwardVector (Variables|Character|GetMesh _self)) (Transformation|GetActorLocation _self)) (Transformation|GetActorRotation _self)))

(event Custom|RotateTowardsPlayer
  (bind _returnvalue (Transformation|GetActorRotation))
  ;[1 0.3105 0.6202] More Accurate Attack
  (Transformation|SetActorRotation (Math|Rotator|MakeRotator (.roll _returnvalue) (.pitch _returnvalue) (.yaw (Math|Rotator|FindLookatRotation (Transformation|GetActorLocation) (Transformation|GetActorLocation (Game|GetPlayerCharacter 0)))))))

(event Custom|IncrementLoops
  ;[0.2812 0.9901 1] ?????
  (bind _result (Math|Integer|IncrementInt (Variables|Default|GetNumOfLoops))
    (:%20%20
      (bind _output_get (Variables|Default|SetNumOfLoops _result))
      (Development|PrintString (Utilities|String|ToString(Integer) _output_get)))))

(event Custom|AttackLight
  (bind _mesh (Variables|Character|GetMesh))
  ;[0.2693 0.2674 1] Boss Animation Triggers
  (CallFunction|MontageReplicationRPC "/Game/Art/Characters/Enemies/WesternBoss/Animations/Monmtages/Anim_BossLightAttack_Montage.Anim_BossLightAttack_Montage" 1.5 "None" 0 _mesh 0.0 true)
  (Animation|Montage|PlayMontage _mesh "/Game/Art/Characters/Enemies/WesternBoss/Animations/Monmtages/Anim_BossLightAttack_Montage.Anim_BossLightAttack_Montage" 1.5
    (:OnCompleted
      _)
    (:OnInterrupted
      _))
  (Default|CallOnLightAttackEnd))

(event Custom|StunAnim
  (bind _mesh (Variables|Character|GetMesh))
  ;[0.2693 0.2674 1] Boss Animation Triggers
  (CallFunction|MontageReplicationRPC "/Game/Art/Characters/Enemies/WesternBoss/Animations/Monmtages/AM_BossStun.AM_BossStun" 0.75 "None" 0 _mesh 0.0 true)
  (Animation|Montage|PlayMontage _mesh "/Game/Art/Characters/Enemies/WesternBoss/Animations/Monmtages/AM_BossStun.AM_BossStun" 0.75
    (:OnCompleted
      _)
    (:OnInterrupted
      _))
  (Default|CallOnStunEnd))

(event Custom|Dash
  (Variables|Default|SetIsHeavySpecial true))

(event Custom|Charging
  (bind _mesh (Variables|Character|GetMesh))
  ;[0.2693 0.2674 1] Boss Animation Triggers
  (CallFunction|MontageReplicationRPC "/Game/Art/Characters/Enemies/WesternBoss/Animations/Monmtages/Boss_Charge_Montage.Boss_Charge_Montage" 0.75 "None" 0 _mesh 0.0 true)
  (Animation|Montage|PlayMontage _mesh "/Game/Art/Characters/Enemies/WesternBoss/Animations/Monmtages/Boss_Charge_Montage.Boss_Charge_Montage" 0.75
    (:OnCompleted
      _)
    (:OnInterrupted
      _))
  (Default|CallOnChargeEnd))

(event Custom|AttackHeavy
  (bind _mesh (Variables|Character|GetMesh))
  (CallFunction|MontageReplicationRPC "/Game/Art/Characters/Enemies/WesternBoss/Animations/Monmtages/Anim_BossHeavyAttack_Part1_Montage.Anim_BossHeavyAttack_Part1_Montage" 1.2 "None" 0 _mesh 0.0 true)
  (Animation|Montage|PlayMontage _mesh "/Game/Art/Characters/Enemies/WesternBoss/Animations/Monmtages/Anim_BossHeavyAttack_Part1_Montage.Anim_BossHeavyAttack_Part1_Montage" 1.2
    (:OnCompleted
      _)
    (:OnInterrupted
      _))
  (Default|CallOnHeavyAttackEnd))

(event Custom|DashFinish
  (Variables|Default|SetIsHeavySpecial false))

(event Custom|AttackSlice
  (bind _self self)
  (bind _mesh (Variables|Character|GetMesh))
  (bind _returnvalue (Transformation|GetActorLocation _self))
  ;[1 0.3503 0.4806] Attack Slice
  (CallFunction|MontageReplicationRPC "/Game/Art/Characters/Enemies/WesternBoss/Animations/Monmtages/BossSpecialAtk/AM_SlowUpChargeKick.AM_SlowUpChargeKick" 1.0 "None" 0 _mesh 0.0 true)
  (Animation|Montage|PlayMontage _mesh "/Game/Art/Characters/Enemies/WesternBoss/Animations/Monmtages/BossSpecialAtk/AM_SlowUpChargeKick.AM_SlowUpChargeKick"
    (:OnCompleted
      _)
    (:OnInterrupted
      _))
  (Niagara|SpawnSystematLocation "/Game/Art/VFX/NS_Dash.NS_Dash" _returnvalue (Transformation|GetActorRotation _self))
  (Audio|PlaySoundatLocation "/Game/Art/SFX/Wooshes/SW_Woosh2.SW_Woosh2" _returnvalue "0, 0, 0" 1.0 1.0 0.0 0 0 0 0)
  (Default|CallOnSliceAttackEnd))

(fn ConstructionScript)

(fn AttackStart
  (params (AttackTarget :type Actor%20Object%20Reference) (Tokens%20Needed :type Integer))
  (return false))

(fn GetIdealRange
  (return 1.2e+02 9e+02 7e+02))

(fn SetMovementSpeed
  (params (Speed :type E_MovementSpeed%20Enum :default "NewEnumerator0"))
  (bind _output_get (Variables|/Script/Engine.CharacterMovementComponent|SetMaxWalkSpeed (Variables|Character|GetCharacterMovement) (Utilities|Select :Index Speed :NewEnumerator0 0.0 :NewEnumerator1 1e+02 :NewEnumerator2 6e+02 :NewEnumerator4 2e+03)))
  (return _output_get))